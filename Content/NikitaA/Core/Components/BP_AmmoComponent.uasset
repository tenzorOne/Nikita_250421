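; BP_AmmoComponent is an ammo-tracking component that holds a current and maximum ammo count.
; On BeginPlay it fills current ammo to the maximum.
; Functions subtract ammo with a clamp between zero and the maximum, check whether enough ammo remains for a given amount, and return both current and max values.
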(event `self.ReceiveBeginPlay`
  (set `self.CurrentAmmo` (`self.MaxAmmo`)))

(fn `CheckAmmo`
  (params (AmmoValue :type Integer :default 1))
  (returns (AmmoAvailable :type Boolean))
  (return (>= (`self.CurrentAmmo`) AmmoValue)))

(fn `GetAmmo`
  (returns (CurrentAmmo :type Integer) (MaxAmmo :type Integer))
  (return (`self.CurrentAmmo`) (`self.MaxAmmo`)))

(fn `Subtract Ammo`
  (params (AmmoValue :type Integer :default 1))
  (set `self.CurrentAmmo` (`KismetMathLibrary.Clamp` (- (`self.CurrentAmmo`) AmmoValue) 0 (`self.MaxAmmo`))))