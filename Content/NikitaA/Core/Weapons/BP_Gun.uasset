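; BP_Gun is a gun actor that a BP_BaseCharacter picks up through its Interact event.
; AttachWeapon turns off mesh physics and collision, then snaps the gun to the character's ActorAttachLocation, keeping relative scale.
; The character cast follows the physics change, so a non-character interactor still leaves physics and collision off.
; DetachWeapon releases the gun in world space and restores both, but nothing here calls it.
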(event `/Game/NikitaA/Core/Interfaces/BPI_Interaction.Interact`
  (params (InteractedFor :type "Actor Object Reference"))
  (`self.AttachWeapon` InteractedFor))

(fn `AttachWeapon`
  (params (ActorToAttach :type "Actor Object Reference"))
  (`PrimitiveComponent.SetSimulatePhysics` (`self.WeaponMesh`) false)
  (`PrimitiveComponent.SetCollisionEnabled` (`self.WeaponMesh`) "NoCollision")
  (bind _asbp_base_character (cast `/Game/NikitaA/Core/Characters/BP_BaseCharacter` ActorToAttach))
  (`self.K2_AttachToComponent` (`/Game/NikitaA/Core/Characters/BP_BaseCharacter.ActorAttachLocation` _asbp_base_character) "None" "SnapToTarget" "SnapToTarget" "KeepRelative"))

(fn `DetachWeapon`
  (`self.K2_DetachFromActor` "KeepWorld" "KeepWorld")
  (`PrimitiveComponent.SetSimulatePhysics` (`self.WeaponMesh`) true)
  (`PrimitiveComponent.SetCollisionEnabled` (`self.WeaponMesh`) "QueryAndPhysics"))

(fn `UserConstructionScript`
  (`parent.UserConstructionScript`))