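; Base lamp actor that randomly switches its light off and on, taking a new random color each time it relights.
; The Construction Script applies exposed color, intensity, radius and shadow settings to the light and lamp material.
; BeginPlay creates a dynamic material instance, starts the lamp lit or dark at even odds, then enters an endless random-delay loop.
; SwitchEmissiveColor keeps material glow synced with light intensity, while the loop copies each new color to the emissive parameter.
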(event `Event Repeat Logic`
  ;[0.7255 1 0.2314] В случайном промежутке времени выключить лампу и снова активировать её + случайная смена цвета источника освещения
  (`KismetSystemLibrary.Delay` (`KismetMathLibrary.RandomFloatInRange` 0.5 3.5) :!label _label)
  (`LightComponent.SetIntensity` (`self.Light`) 0.0)
  (`self.SwitchEmissiveColor`)
  (`KismetSystemLibrary.Delay` (`KismetMathLibrary.RandomFloatInRange` 0.25 3.0))
  (`LightComponent.SetIntensity` (`self.Light`) (`self.Intensity`))
  (`self.SwitchEmissiveColor`)
  (`LightComponent.SetLightColor` (`self.Light`) (`KismetMathLibrary.MakeColor` (`KismetMathLibrary.RandomFloatInRange` 0.0 1.0) (`KismetMathLibrary.RandomFloatInRange` 0.0 1.0) (`KismetMathLibrary.RandomFloatInRange` 0.0 1.0)) true)
  (`MaterialInstanceDynamic.SetVectorParameterValue` (`self.DMI`) "ColorEmissive" (`LightComponentBase.GetLightColor` (`self.Light`)))
  (`self.Event Repeat Logic`))

(event `self.ReceiveBeginPlay`
  ;[1 0.1771 0.1771] Создать динамический инстанс материала
  (bind _returnvalue (`PrimitiveComponent.CreateDynamicMaterialInstance` (`self.LampMesh`) 0 "/Game/StarterContent/Props/Materials/M_Lamp.M_Lamp" "None"))
  (set `self.DMI` _returnvalue)
  ;[0.7255 1 0.2314] При старте игры (симуляции) с вероятностью 50% отключить лампу
  (`LightComponent.SetIntensity` (`self.Light`) (`KismetMathLibrary.SelectFloat` (`self.Intensity`) 0.0 (`KismetMathLibrary.RandomBoolWithWeight` 0.5)))
  ;[0.7255 1 0.2314] Когда интенсивность источника освещения равна нулю,
  ; то изменить значение Emissive Color внутри материала лампы на ноль
  (`self.SwitchEmissiveColor`)
  (goto _label))

(fn `SwitchEmissiveColor`
  (bind _dmi (`self.DMI`))
  (if (== (`LightComponentBase.Intensity` (`self.Light`)) 0.0)
    (`MaterialInstanceDynamic.SetScalarParameterValue` _dmi "Glow" 0.0)
    (else
      (`MaterialInstanceDynamic.SetScalarParameterValue` _dmi "Glow" 5.0))))

(fn `UserConstructionScript`
  (bind _lampmesh (`self.LampMesh`))
  ;[1 1 1] Публичные параметры экземпляра класса
  (`LightComponent.SetLightColor` (`self.Light`) (`self.Color`) true)
  (`MeshComponent.SetVectorParameterValueOnMaterials` (`self.LampMesh`) "ColorEmissive" (`KismetMathLibrary.Conv_LinearColorToVector` (`self.Color`)))
  (`LightComponent.SetIntensity` (`self.Light`) (`self.Intensity`))
  (`LocalLightComponent.SetAttenuationRadius` (`self.Light`) (`self.Radius`))
  (`LightComponentBase.SetCastShadows` (`self.Light`) (`self.CastShadows`))
  ;[1 1 1] Когда интенсивность источника освещения равна нулю,
  ; то изменить значение Emissive Color внутри материала лампы на ноль
  (if (== (`LightComponentBase.Intensity` (`self.Light`)) 0.0)
    (`MeshComponent.SetScalarParameterValueOnMaterials` _lampmesh "Glow" 0.0)
    (else
      (`MeshComponent.SetScalarParameterValueOnMaterials` _lampmesh "Glow" 5.0))))