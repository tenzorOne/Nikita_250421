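; BP_Button is an interactable button that toggles its screen material and light between green and red and activates linked lamps.
; Interact flips the colour and calls ButtonActivate on every lamp in LampReferences.
; A DoOnce inside that loop sets LampEnabled only on the first lamp processed.
; Character overlaps toggle the Info component's visibility, while the code registering the button for interaction is disconnected.
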(event `self.ButtonTrigger.OnComponentBeginOverlap`
  (params (OverlappedComponent :type "PrimitiveComponent Object Reference") (OtherActor :type "Actor Object Reference") (OtherComp :type "PrimitiveComponent Object Reference") (OtherBodyIndex :type Integer) (bFromSweep :type Boolean) (SweepResult :type "HitResult Structure (by ref)"))
  (bind _asbp_base_character (cast `/Game/NikitaA/Core/Characters/BP_BaseCharacter` OtherActor))
  (`SceneComponent.ToggleVisibility` (`self.Info`) false))

(event `self.ButtonTrigger.OnComponentEndOverlap`
  (params (OverlappedComponent :type "PrimitiveComponent Object Reference") (OtherActor :type "Actor Object Reference") (OtherComp :type "PrimitiveComponent Object Reference") (OtherBodyIndex :type Integer))
  (bind _asbp_base_character (cast `/Game/NikitaA/Core/Characters/BP_BaseCharacter` OtherActor))
  (`SceneComponent.ToggleVisibility` (`self.Info`) false))

(event `/Game/NikitaA/Core/Interfaces/BPI_Interaction.Interact`
  (`/Engine/EditorBlueprintResources/StandardMacros.FlipFlop`
    (:`A`
      (`MaterialInstanceDynamic.SetVectorParameterValue` (`self.DMI`) "Color" (struct :`G` 1.0 :`A` 1.0))
      (`LightComponent.SetLightColor` (`self.ButtonLight`) (struct :`G` 1.0 :`A` 1.0) true))
    (:`B`
      (`MaterialInstanceDynamic.SetVectorParameterValue` (`self.DMI`) "Color" (struct :`R` 1.0 :`A` 1.0))
      (`LightComponent.SetLightColor` (`self.ButtonLight`) (struct :`R` 1.0 :`A` 1.0) true)))
  (for _array_element (`self.LampReferences`)
    (`|ExecutionSequence`
      (:`then_0`
        (`/Engine/EditorBlueprintResources/StandardMacros.DoOnce` false
          (:`Completed`
            (set `/Game/NikitaA/Interactable/BP_BaseLamp.LampEnabled` true _array_element))))
      (:`then_1`
        (`/Game/NikitaA/Interactable/BP_BaseLamp.ButtonActivate` _array_element)))))

(fn `UserConstructionScript`
  (bind _returnvalue (`PrimitiveComponent.CreateDynamicMaterialInstance` (`self.ButtonMesh`) 0 "/Game/NikitaA/Materials/M_ButtonScreen.M_ButtonScreen" "None"))
  (set `self.DMI` _returnvalue))