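; BP_Door is a door actor that swings open and closed on its own in an endless loop, with no player input.
; Tick eases the Door component's relative rotation with RInterpTo toward either a random negative yaw or zero, depending on the Open flag.
; Reaching the open angle flips the flag after a short random Delay, while reaching closed flips it immediately and rolls a new angle.
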(event `self.ReceiveBeginPlay`
  ;[0.1985 0.6274 1] Инициализация случайного вращения по Yaw (Z)
  (set `self.RandomRotator` (`KismetMathLibrary.NegateRotator` (`KismetMathLibrary.MakeRotator` 0.0 0.0 (`KismetMathLibrary.RandomFloatInRange` 1.0 80.0)))))

(event `self.ReceiveTick`
  (params (DeltaSeconds :type "Float (single-precision)"))
  (if (`self.Open`)
    ;[1 1 1] Открытие двери
    (`SceneComponent.K2_SetRelativeRotation` (`self.Door`) (`KismetMathLibrary.RInterpTo` (`SceneComponent.RelativeRotation` (`self.Door`)) (`self.RandomRotator`) (`GameplayStatics.GetWorldDeltaSeconds`) 1.0) false false) ; Интерполяция до нужного значения
    (if (== (`SceneComponent.RelativeRotation` (`self.Door`)) (`self.RandomRotator`) :`ErrorTolerance` 0.5)
      (`KismetSystemLibrary.Delay` (`KismetMathLibrary.RandomFloatInRange` 0.2 2.0)) ; Через небольшой промежуток времени позволить двери закрыться
      (set `self.Open` false))
    (else
      ;[1 1 1] Закрытие двери
      (`SceneComponent.K2_SetRelativeRotation` (`self.Door`) (`KismetMathLibrary.RInterpTo` (`SceneComponent.RelativeRotation` (`self.Door`)) (struct) (`GameplayStatics.GetWorldDeltaSeconds`) 1.0) false false) ; Интерполяция до нужного значения
      (if (== (`SceneComponent.RelativeRotation` (`self.Door`)) (struct) :`ErrorTolerance` 0.5)
        (set `self.Open` true) ; Позволить двери открыться
        (set `self.RandomRotator` (`KismetMathLibrary.NegateRotator` (`KismetMathLibrary.MakeRotator` 0.0 0.0 (`KismetMathLibrary.RandomFloatInRange` 1.0 80.0)))) ; Задать новый угол для рандомного поворота
      ))))

(fn `UserConstructionScript`)