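; BP_Turret is a placeable turret that automatically fires from two barrels while it has ammo, with no targeting logic in its graph.
; A looping one-second timer started on BeginPlay spawns a BP_AmmoBase at the left and right spawn points.
; AmmoComponent gates each volley by checking for one round but subtracting two, and the AmmoCount text shows current and max ammo, refreshed after each volley.
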(event `self.ReceiveBeginPlay`
  (bind (_currentammo _maxammo) (`/Game/NikitaA/Core/Components/BP_AmmoComponent.GetAmmo` (`self.AmmoComponent`)))
  (`TextRenderComponent.K2_SetText` (`self.AmmoCount`) (`|FormatText` "{Current}|{Max}" _currentammo _maxammo))
  (`KismetSystemLibrary.K2_SetTimerDelegate` (delegate `TurretFire`) 1.0 true))

(event `TurretFire`
  (bind (_currentammo _maxammo) (`/Game/NikitaA/Core/Components/BP_AmmoComponent.GetAmmo` (`self.AmmoComponent`)))
  (if (`/Game/NikitaA/Core/Components/BP_AmmoComponent.CheckAmmo` (`self.AmmoComponent`) 1)
    (`/Game/NikitaA/Core/Components/BP_AmmoComponent.Subtract Ammo` (`self.AmmoComponent`) 2)
    (`|SpawnActorFromClass` "/Game/NikitaA/Core/Weapons/BP_AmmoBase.BP_AmmoBase_C" (`SceneComponent.K2_GetComponentToWorld` (`self.LeftAmmoSpawn`)) "AlwaysSpawn" "OverrideRootScale" null null)
    (`|SpawnActorFromClass` "/Game/NikitaA/Core/Weapons/BP_AmmoBase.BP_AmmoBase_C" (`SceneComponent.K2_GetComponentToWorld` (`self.RightAmmoSpawn`)) "AlwaysSpawn" "OverrideRootScale" null null)
    (`TextRenderComponent.K2_SetText` (`self.AmmoCount`) (`|FormatText` "{Current}|{Max}" _currentammo _maxammo))))

(fn `UserConstructionScript`)