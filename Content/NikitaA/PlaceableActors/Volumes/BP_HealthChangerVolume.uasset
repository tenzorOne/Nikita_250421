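; BP_HealthChangerVolume is a placeable zone that periodically heals or damages a character inside it, depending on VolumeType.
; Overlap starts a looping half-second timer that calls the character's CharacterStatusComponent, and end overlap clears it.
; It tracks only one target: each new overlap replaces the stored actor and timer handle.
; The construction script sizes the trigger and tints a dynamic void-zone material green or red by type.
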(event `self.VolumeTrigger.OnComponentBeginOverlap`
  (params (OverlappedComponent :type "PrimitiveComponent Object Reference") (OtherActor :type "Actor Object Reference") (OtherComp :type "PrimitiveComponent Object Reference") (OtherBodyIndex :type Integer) (bFromSweep :type Boolean) (SweepResult :type "HitResult Structure (by ref)"))
  (set `self.TargetActor` OtherActor)
  (bind _returnvalue (`KismetSystemLibrary.K2_SetTimerDelegate` (delegate `VolumeAction`) 0.5 true))
  (set `self.VolumeActionTimer` _returnvalue))

(event `VolumeAction`
  (bind _asbp_base_character (cast `/Game/NikitaA/Core/Characters/BP_BaseCharacter` (`self.TargetActor`)))
  (switch `/Game/NikitaA/PlaceableActors/Volumes/EVolumeType` (`self.VolumeType`)
    (:`NewEnumerator0`
      (bind _characterstatuscomponent (`/Game/NikitaA/Core/Characters/BP_BaseCharacter.CharacterStatusComponent` _asbp_base_character))
      (`/Game/NikitaA/Core/Components/BP_CharacterStatusComponent.Heal` _characterstatuscomponent 2))
    (:`NewEnumerator1`
      (`/Game/NikitaA/Core/Components/BP_CharacterStatusComponent.MakeDamage` _characterstatuscomponent 5))))

(event `self.VolumeTrigger.OnComponentEndOverlap`
  (params (OverlappedComponent :type "PrimitiveComponent Object Reference") (OtherActor :type "Actor Object Reference") (OtherComp :type "PrimitiveComponent Object Reference") (OtherBodyIndex :type Integer))
  (set `self.TargetActor` null)
  (`KismetSystemLibrary.K2_ClearAndInvalidateTimerHandle` (`self.VolumeActionTimer`)))

(fn `UserConstructionScript`
  (bind _returnvalue (`PrimitiveComponent.CreateDynamicMaterialInstance` (`self.VolumeVisualPlane`) 0 "/Game/NikitaA/Materials/M_VoidZone.M_VoidZone" "None"))
  (set `self.DMI` _returnvalue)
  (`SceneComponent.SetWorldScale3D` (`self.VolumeTrigger`) (`KismetMathLibrary.MakeVector` (`self.TriggerSizeX`) (`self.TriggerSizeY`) 1.0))
  (switch `/Game/NikitaA/PlaceableActors/Volumes/EVolumeType` (`self.VolumeType`)
    (:`NewEnumerator0`
      (`MaterialInstanceDynamic.SetVectorParameterValue` (`self.DMI`) "Color" (struct :`G` 1.0 :`A` 1.0)))
    (:`NewEnumerator1`
      (`MaterialInstanceDynamic.SetVectorParameterValue` (`self.DMI`) "Color" (struct :`R` 1.0 :`A` 1.0)))))